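; Game mode for MarsMarine that runs endless, escalating waves of BP_Alien spiders, starting shortly after BeginPlay.
; Each wave scales the spider count and spawn interval by multipliers, then a looping timer spawns aliens at random TargetPoints until none remain to spawn.
; RegisterSpiderDeath removes spiders from the tracked array and, once it is empty with no spawns pending, starts the next wave after a short delay.
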(event `self.ReceiveBeginPlay`
  (`KismetSystemLibrary.Delay` 2.5)
  (`self.Start New Wave`))

(event `Spawn Wave`
  (`self.Spawn Spiders`))

(event `End Wave`
  (`KismetSystemLibrary.Delay` 2.0)
  (`self.Start New Wave`))

(fn `Get Random Spawn Point`
  (returns (`Spawn Point` :type "TargetPoint Object Reference"))
  (bind _outactors (`GameplayStatics.GetAllActorsOfClass` "/Script/Engine.TargetPoint"))
  (return (`|GetArrayItem` _outactors (`KismetMathLibrary.RandomIntegerInRange` 0 (`KismetArrayLibrary.Array_LastIndex` _outactors)))))

(fn `Increase Wave Diffuculty`
  (bind _output_get (set `self.Wave Difficulty` (`KismetMathLibrary.Round` (* (`self.Wave Difficulty`) (`self.Difficulty Multiplier`)))))
  (set `self.Spider Spawns Remaining` _output_get)
  (bind _output_get_2 (set `self.Spawn Frequency` (* (`self.Spawn Frequency`) (`self.Spawn Frequency Multiplier`))))
  (`KismetSystemLibrary.PrintString` (`KismetStringLibrary.Conv_DoubleToString` _output_get_2)))

(fn `Is Wave Complete`
  (returns (ReturnValue :type Boolean))
  (return (and (== (`KismetArrayLibrary.Array_Length` (`self.Spiders`)) 0) (== (`self.Spider Spawns Remaining`) 0))))

(fn `Register Spider Death`
  (params (Spiders :type "/Game/Blueprints/AI/BP_Alien Object Reference (by ref)"))
  (`KismetArrayLibrary.Array_RemoveItem` (`self.Spiders`) Spiders)
  (if (`self.Is Wave Complete`)
    (`self.End Wave`)))

(fn `Spawn Spiders`
  (bind _spawn_point (`self.Get Random Spawn Point`))
  (`/Engine/EditorBlueprintResources/StandardMacros.IsValid` _spawn_point
    (:`Is Valid`
      (bind _returnvalue (`|SpawnActorFromClass` "/Game/Blueprints/AI/BP_Alien.BP_Alien_C" (`self.GetTransform` _spawn_point) "Undefined" "OverrideRootScale" null null))
      (`/Engine/EditorBlueprintResources/StandardMacros.IsValid` _returnvalue
        (:`Is Valid`
          (`KismetArrayLibrary.Array_Add` (`self.Spiders`) _returnvalue)
          (bind _result (`/Engine/EditorBlueprintResources/StandardMacros.DecrementInt` (`self.Spider Spawns Remaining`))
            (:`  `
              (if (== _result 0)
                (`KismetSystemLibrary.K2_ClearTimer` null "Spawn Wave")))))))))

(fn `Start New Wave`
  (`/Engine/EditorBlueprintResources/StandardMacros.IncrementInt` (`self.Current Wave`)
    (:`  `
      (`self.Increase Wave Diffuculty`)
      (`KismetSystemLibrary.K2_SetTimer` null "Spawn Wave" (`self.Spawn Frequency`) true))))

(fn `UserConstructionScript`)