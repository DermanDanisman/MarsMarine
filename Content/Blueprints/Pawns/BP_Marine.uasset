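; BP_Marine is the player marine pawn, with world-axis movement, twin-stick-style aiming, health and a HUD widget.
; Each tick it sets control yaw from gamepad thumbstick or smoothed mouse velocity, both deadzone-filtered, switching on the last key's device.
; Firing only toggles muzzle flash and rifle audio, with no shot or hit logic here.
; Damage drains health until death, which stops firing and blocks movement and aiming.
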(event `InputAction|Fire Weapon`
  (params (Key :type "Key Structure"))
  ;[1 1 1] Weapon Firing Input
  (:`Pressed`
    (`self.Start Firing Weapon`))
  (:`Released`
    (`self.Stop Firing Weapon`)))

(event `InputAxis|Move_Forward&Backward`
  (params (AxisValue :type "Float (single-precision)"))
  ;[1 1 1] Movement
  (if (`self.Is Alive`)
    (`self.AddMovementInput` (1.0 0.0 0.0) AxisValue)))

(event `InputAxis|Move_Right&Left`
  (params (AxisValue :type "Float (single-precision)"))
  ;[1 1 1] Movement
  (if (`self.Is Alive`)
    (`self.AddMovementInput` (0.0 1.0 0.0) AxisValue)))

(event `self.ReceiveBeginPlay`
  ;[1 1 1] HUD
  (bind _returnvalue (`|CreateWidget` "/Game/UI/W_PlayerHUD.W_PlayerHUD_C" null self))
  (`UserWidget.AddToViewport` _returnvalue 0))

(event `self.ReceiveTick`
  (params (DeltaSeconds :type "Float (single-precision)"))
  ;[1 1 1] Aim Controller
  (if (`self.Is Alive`)
    (`self.Update Player Aim`)))

(event `Key|AnyKey`
  (params (Key :type "Key Structure"))
  ;[1 1 1] Aim Controller
  (:`Pressed`
    (set `self.Is Gamepad Active` (`KismetInputLibrary.Key_IsGamepadKey` Key))))

(event `self.ReceiveAnyDamage`
  (params (Damage :type "Float (single-precision)") (DamageType :type "DamageType Object Reference") (InstigatedBy :type "Controller Object Reference") (DamageCauser :type "Actor Object Reference"))
  ;[1 1 1] Player Get Damage
  (bind _health (`self.Decrease Health` Damage))
  (if (<= _health 0.0)
    (set `self.Is Dead` true)
    (`self.Stop Firing Weapon`)))

(fn `Decrease Health`
  (params (B :type "Float (double-precision)"))
  (returns (Health :type "Float (double-precision)"))
  (bind _output_get (set `self.Marine Health` (- (`self.Marine Health`) B)))
  (return _output_get))

(fn `Get Mouse Aim Direction`
  (returns (ReturnValue :type "Rotator Structure"))
  (bind (_returnvalue_x _returnvalue_y) (`KismetMathLibrary.BreakVector2D` (`self.Get Mouse Velocity`)))
  (return (`KismetMathLibrary.RInterpTo` (`Controller.GetControlRotation` (`GameplayStatics.GetPlayerController` 0)) (`KismetMathLibrary.MakeRotator` 0.0 0.0 (`KismetMathLibrary.DegAtan2` _returnvalue_x _returnvalue_y)) (`GameplayStatics.GetWorldDeltaSeconds`) (`self.Mouse Smoothing Strength`))))

(fn `Get Mouse Velocity`
  (returns (ReturnValue :type "Vector2D Structure"))
  (bind (_deltax _deltay) (`PlayerController.GetInputMouseDelta` (`GameplayStatics.GetPlayerController` 0)))
  (return (/ (`KismetMathLibrary.MakeVector2D` _deltax _deltay) (`GameplayStatics.GetWorldDeltaSeconds`))))

(fn `Get Thumbsick Aim Direction`
  (returns (ReturnValue :type "PlayerController Object Reference") (ReturnValue2 :type "Rotator Structure"))
  (return (`GameplayStatics.GetPlayerController` 0) (`KismetMathLibrary.MakeRotator` 0.0 0.0 (`KismetMathLibrary.DegAtan2` (`self.GetInputAxisValue`) (`self.GetInputAxisValue`)))))

(fn `Is Alive`
  (returns (ReturnValue :type Boolean))
  (return (not (`self.Is Dead`))))

(fn `Is Mouse Above Deadzone`
  (returns (`Return Value` :type Boolean))
  (return (> (`KismetMathLibrary.VSize2D` (`self.Get Mouse Velocity`)) (`self.Mouse Deadzone`))))

(fn `Is Thumbstick Above Deadzone`
  (returns (`Return Value` :type Boolean))
  (return (> (`KismetMathLibrary.VSize2D` (`KismetMathLibrary.MakeVector2D` (`self.GetInputAxisValue`) (`self.GetInputAxisValue`))) (`self.Thumbstick Deadzone`))))

(fn `Start Firing Weapon`
  (if (`self.Is Alive`)
    (`ActorComponent.Activate` (`self.Muzzle Flash`) false)
    (bind _returnvalue (`GameplayStatics.SpawnSound2D` "/Game/Sounds/Weapon_AssaultRifle/Stereo/RifleFire_SoundCue.RifleFire_SoundCue" 1.0 1.0 0.0 null))
    (set `self.Weapon Fire Sound` _returnvalue)))

(fn `Stop Firing Weapon`
  (bind _weapon_fire_sound (`self.Weapon Fire Sound`))
  (`ActorComponent.Deactivate` (`self.Muzzle Flash`))
  (`/Engine/EditorBlueprintResources/StandardMacros.IsValid` _weapon_fire_sound
    (:`Is Valid`
      (`AudioComponent.Stop` _weapon_fire_sound)
      (if (`self.Is Alive`)
        (`GameplayStatics.SpawnSound2D` "/Game/Sounds/Weapon_AssaultRifle/Stereo/RifleFireEnd_SoundCue.RifleFireEnd_SoundCue" 1.0 1.0 0.0 null)))))

(fn `Update Mouse Aim`
  (if (`self.Is Mouse Above Deadzone`)
    (`Controller.SetControlRotation` (`GameplayStatics.GetPlayerController` 0) (`self.Get Mouse Aim Direction`))))

(fn `Update Player Aim`
  (if (`self.Is Gamepad Active`)
    (`self.Update Thumbstick Aim`)
    (else
      (`self.Update Mouse Aim`))))

(fn `Update Thumbstick Aim`
  (bind (_returnvalue _returnvalue2) (`self.Get Thumbsick Aim Direction`))
  (if (`self.Is Thumbstick Above Deadzone`)
    (`Controller.SetControlRotation` _returnvalue _returnvalue2)))

(fn `UserConstructionScript`)